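; BP_PolarBear is a companion bear that follows BP_PlayerCharacter by having its location set directly every Tick, without sweep or pathfinding.
; Tick caches the player's location and a point behind the PlayerModel's forward vector, then PolarMove places the bear there plus DistanceFromCharacter.
; When FollowingPlayer is false it snaps to GivenLocationBear instead, though this graph only sets that flag true.
; The PolarBearInteract input toggles StopFollow to freeze or resume movement, printing debug strings.
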(event Custom|PolarMove
  (if (not (Variables|Default|GetStop%20Follow))
    (if (Variables|Default|GetFollowingPlayer?)
      (Transformation|SetActorLocation (+ (Variables|Default|GetPlayerLocation) (Variables|Default|GetPlayerFacing) (Variables|Default|GetDistance%20From%20Character)) false false)
      (else
        (Transformation|SetActorLocation (Variables|Default|GetGivenLocationBear) false false)))))

(event EventBeginPlay
  ;[1 1 1] Sets the player character to the bp_playercharacter
  (bind _returnvalue (Actor|GetActorOfClass "/Game/Blueprints/Characters/BP_PlayerCharacter.BP_PlayerCharacter_C"))
  (Variables|Default|SetPlayerCharacter _returnvalue)
  (Variables|Default|SetFollowingPlayer? true)
  (Variables|Default|SetStop%20Follow false))

(event EventTick
  (params (DeltaSeconds :type Float%20%28single-precision%29))
  ;[1 1 1] Checking the playable characters location and setting it to premade varibales in order for them to be accessible with ease throughout the blueprint/code
  (Variables|Default|SetPlayerLocation (Transformation|GetActorLocation (Variables|Default|GetPlayerCharacter)))
  (bind _asbp_player_character (Utilities|Casting|CastToBP_PlayerCharacter (Variables|Default|GetPlayerCharacter)))
  (Variables|Default|SetPlayerFacing (* (Math|Vector|GetForwardVector (Variables|/Game/Blueprints/Characters/BP_PlayerCharacter.BP_PlayerCharacter_C|GetPlayerModel _asbp_player_character)) -1.8e+02))
  (CallFunction|PolarMove))

(event Input|ActionEvents|InputActionPolarBearInteract
  (params (Key :type Key%20Structure :default "None"))
  (:Pressed
    (if (Variables|Default|GetStop%20Follow)
      (Variables|Default|SetStop%20Follow false)
      (Development|PrintString "cats" true true "(R=1.000000,G=0.000000,B=0.241413,A=1.000000)")
      (else
        (Variables|Default|SetStop%20Follow true)
        (Development|PrintString "dogs" true true "(R=0.758574,G=1.000000,B=0.457433,A=1.000000)")))))

(fn ConstructionScript)