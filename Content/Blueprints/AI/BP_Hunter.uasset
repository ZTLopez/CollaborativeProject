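; BP_Hunter is an AI hunter that roams and detects nearby player characters or polar bears.
; AIMOVE picks an offset target, fixed rather than random because each range's min and max match, and a Timeline drives movement input toward it.
; Each update runs two sphere overlaps: exactly one hit type sets IsInRadius, otherwise a delayed AIMOVE picks a new target.
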(event Custom|AI%20MOVE
  (bind _hunterbase (Variables|Default|GetHunterBase))
  (bind _returnvalue (Transformation|GetWorldLocation _hunterbase))
  (Variables|Default|SetnewLocation (Math|Vector|MakeVector (+ (Math|Random|RandomFloatinRange (Variables|Default|GetRandom%20Number%20X+) (Variables|Default|GetRandom%20Number%20X-)) (.x _returnvalue)) (+ (.y _returnvalue) (Math|Random|RandomFloatinRange (Variables|Default|GetRandom%20Number%20Y+) (Variables|Default|GetRandom%20Number%20Y-))) (.z _returnvalue)))
  (Timeline|Movement PlayFromStart
    (:Update
      (Pawn|Input|AddMovementInput (Math|Vector|Normalize (- (Variables|Default|GetnewLocation) (Transformation|GetWorldLocation (Variables|Default|GetHunterBase)))) 0.4 false)
      (CallFunction|CheckRadius))))

(event Custom|Check%20Radius
  (bind _array (Utilities|Array|MakeArray "ObjectTypeQuery3" "ObjectTypeQuery2"))
  (bind _huntercollision (Variables|Default|GetHunterCollision))
  (bind _returnvalue (Transformation|GetWorldLocation _huntercollision))
  (bind _returnvalue_2 (Collision|SphereOverlapActors _returnvalue 1e+02 _array "/Game/Blueprints/Characters/BP_PlayerCharacter.BP_PlayerCharacter_C"))
  (bind _returnvalue_3 (Collision|SphereOverlapActors _returnvalue 1e+02 _array "/Game/Blueprints/AI/BP_PolarBear.BP_PolarBear_C"))
  (if (Class|KismetMathLibrary|XORBoolean _returnvalue_2 _returnvalue_3)
    (Development|PrintString "Found PLayer")
    (Variables|Default|SetIs%20In%20Radius? true)
    (else
      (Utilities|FlowControl|Delay 2.0)
      (CallFunction|AIMOVE))))

(event EventBeginPlay
  (Components|Timeline|SetPlayRate (Variables|Default|GetMovement) (Variables|Default|GetHunter%20Speed))
  (CallFunction|AIMOVE))

(fn ConstructionScript)