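; BP_ThinIce is an interactable thin-ice trigger that stages a short scripted player crossing with the polar bear when the player overlaps it.
; BeginPlay caches the player, bear and marker component positions, though the bear's end position goes unused.
; On overlap it snaps both characters to their start markers, disables input, and a timeline lerps the player's X/Y to the end point.
; A delay chained from the timeline update restores input and destroys the actor.
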(event EventBeginPlay
  (Variables|Default|SetStartposition (Transformation|GetWorldLocation (Variables|Default|GetPlayerPosition)))
  (Variables|Default|SetBear%20position (Transformation|GetWorldLocation (Variables|Default|Getbearlocation)))
  (bind _returnvalue (Actor|GetActorOfClass "/Game/Blueprints/Characters/BP_PlayerCharacter.BP_PlayerCharacter_C"))
  (Variables|Default|Setplayercharacter _returnvalue)
  (Variables|Default|Setendpositionplayer (Transformation|GetWorldLocation (Variables|Default|Getendpointplayer)))
  (bind _returnvalue_2 (Actor|GetActorOfClass "/Game/Blueprints/AI/BP_PolarBear.BP_PolarBear_C"))
  (Variables|Default|Setbearcharacter _returnvalue_2)
  (Variables|Default|Setendpositionbear (Transformation|GetWorldLocation (Variables|Default|Getendpointbear))))

(event Collision|EventActorBeginOverlap
  (params (OtherActor :type Actor%20Object%20Reference))
  (bind _returnvalue (Game|GetPlayerController 0))
  (bind _playercharacter (Variables|Default|Getplayercharacter))
  (bind _playercharacter_2 (Variables|Default|Getplayercharacter))
  (bind _startposition (Variables|Default|GetStartposition))
  (bind _endpositionplayer (Variables|Default|Getendpositionplayer))
  (bind _returnvalue_2 (Transformation|GetActorLocation _playercharacter_2))
  (if (== OtherActor (Variables|Default|Getplayercharacter))
    (Transformation|SetActorRelativeLocation (Variables|Default|Getplayercharacter) (Variables|Default|GetStartposition))
    (Transformation|SetActorRelativeLocation (Variables|Default|Getbearcharacter) (Variables|Default|GetBear%20position))
    (Input|DisableInput _playercharacter _returnvalue)
    (Utilities|FlowControl|Delay 0.5)
    (bind _moveto (Timeline|moveto Play)
      (:Update
        (Transformation|SetActorRelativeLocation _playercharacter (Math|Vector|Lerp(Vector) (Math|Vector|MakeVector (.x _startposition) (.y _startposition) (.z _returnvalue_2)) (Math|Vector|MakeVector (.x _endpositionplayer) (.y _endpositionplayer) (.z _returnvalue_2)) _moveto))
        (Utilities|FlowControl|Delay 5.0)
        (Input|EnableInput _playercharacter _returnvalue)
        (Actor|DestroyActor)))))

(fn ConstructionScript)