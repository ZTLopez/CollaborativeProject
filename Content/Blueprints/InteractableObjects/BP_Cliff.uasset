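; BP_Cliff is an interactable cliff that moves the player character to a preset end point on overlap.
; BeginPlay caches the player character and the world location of its EndCollision component.
; When the player overlaps, it disables input, waits five seconds, sets the player's relative location to that cached end location without sweeping, then restores input.
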(event EventBeginPlay
  (Variables|Default|Setendlocation (Transformation|GetWorldLocation (Variables|Default|Getend%20Collision)))
  (bind _returnvalue (Actor|GetActorOfClass "/Game/Blueprints/Characters/BP_PlayerCharacter.BP_PlayerCharacter_C"))
  (Variables|Default|Setplayercharacter _returnvalue))

(event Collision|EventActorBeginOverlap
  (params (OtherActor :type Actor%20Object%20Reference))
  (Utilities|Casting|CastToBP_PlayerCharacter OtherActor)
  (Input|DisableInput (Variables|Default|Getplayercharacter) (Game|GetPlayerController 0))
  (Utilities|FlowControl|Delay 5.0)
  (Transformation|SetActorRelativeLocation (Variables|Default|Getplayercharacter) (Variables|Default|Getendlocation))
  (Input|EnableInput (Variables|Default|Getplayercharacter) (Game|GetPlayerController 0)))

(event EventTick
  (params (DeltaSeconds :type Float%20%28single-precision%29)))

(fn ConstructionScript)