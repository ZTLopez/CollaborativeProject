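; BP_Rock is an interactable rock that the polar bear pushes aside once.
; Until moved, an overlap stops the bear following, disables player input and teleports both characters to marker positions.
; If the overlapping actor is the bear, a timeline slides the rock collision along X after a short delay, keeping the bear on its push point.
; On completion, input and following resume and the rock is flagged as moved.
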(event Custom|MoveRock
  (bind _movement (Timeline|Movement Play)
    (:Update
      (Transformation|SetRelativeLocation (Variables|Default|GetRockCollision) (Math|Vector|MakeVector (Math|Float|Lerp 0.0 -1e+02 _movement) 0.0 0.0) false false)
      (bind _output_get (Variables|/Game/Blueprints/AI/BP_PolarBear.BP_PolarBear_C|SetGivenLocationBear (Variables|Default|GetBearCharacterActor) (Transformation|GetWorldLocation (Variables|Default|GetBearmoveto))))
      (Transformation|SetRelativeLocation (Variables|/Script/Engine.Actor|GetRootComponent (stale Collision|EventActorBeginOverlap _asbp_polar_bear)) _output_get false false))
    (:Finished
      (Input|EnableInput (Variables|Default|GetPlayerCharacter) (Game|GetPlayerController 0))
      (Variables|/Game/Blueprints/AI/BP_PolarBear.BP_PolarBear_C|SetFollowingPlayer? (Variables|Default|GetBearCharacterActor) true)
      (Variables|Default|SetHas%20been%20moved true))))

(event EventBeginPlay
  (Variables|Default|SetHas%20been%20moved false)
  (Variables|Default|SetBear%20Push%20Point (Transformation|GetWorldLocation (Variables|Default|GetBearmoveto)))
  (bind _returnvalue (Actor|GetActorOfClass "/Game/Blueprints/Characters/BP_PlayerCharacter.BP_PlayerCharacter_C"))
  (Variables|Default|SetPlayerCharacter _returnvalue)
  (bind _returnvalue_2 (Actor|GetActorOfClass "/Game/Blueprints/AI/BP_PolarBear.BP_PolarBear_C"))
  (bind _output_get (Variables|Default|SetBearCharacterActor _returnvalue_2))
  (Variables|/Game/Blueprints/AI/BP_PolarBear.BP_PolarBear_C|SetGivenLocationBear _output_get (Variables|Default|GetBear%20Push%20Point))
  (Variables|Default|SetPlayerstance (Transformation|GetWorldLocation (Variables|Default|GetPlayerStand))))

(event Collision|EventActorBeginOverlap
  (params (OtherActor :type Actor%20Object%20Reference))
  (if (not (Variables|Default|GetHas%20been%20moved))
    (Variables|/Game/Blueprints/AI/BP_PolarBear.BP_PolarBear_C|SetFollowingPlayer? (Variables|Default|GetBearCharacterActor) false)
    (Input|DisableInput (Variables|Default|GetPlayerCharacter) (Game|GetPlayerController 0))
    (Transformation|SetActorRelativeLocation (Variables|Default|GetPlayerCharacter) (Variables|Default|GetPlayerstance))
    (Transformation|SetActorRelativeLocation (Variables|Default|GetBearCharacterActor) (Variables|Default|GetBear%20Push%20Point))
    (bind _asbp_polar_bear (Utilities|Casting|CastToBP_PolarBear OtherActor))
    (Utilities|FlowControl|Delay 1.0)
    (CallFunction|MoveRock)))

(fn ConstructionScript)